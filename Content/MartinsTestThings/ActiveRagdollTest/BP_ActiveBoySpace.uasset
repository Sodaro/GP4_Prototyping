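; BP_ActiveBoySpace is an active ragdoll test pawn that the player moves with physics forces.
; Move input pushes the Sphere along control-yaw directions, Jump adds an upward impulse, and Left Shift raises the move force while held.
; Each tick, the Sphere snaps to control yaw and gets a vertical UpForce while both legs get DownForce, apparently to keep the body upright.
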(event `InputAction|Jump`
  (params (Key :type "Key Structure"))
  (:`Pressed`
    (`PrimitiveComponent.AddImpulse` (`self.Sphere`) (0.0 0.0 400000.0) "None" false)))

(event `InputAxis|Look Up / Down Mouse`
  (params (AxisValue :type "Float (single-precision)"))
  (`self.AddControllerPitchInput` AxisValue))

(event `InputAxis|Turn Right / Left Mouse`
  (params (AxisValue :type "Float (single-precision)"))
  (`self.AddControllerYawInput` AxisValue))

(event `InputAxis|Move Forward / Backward`
  (params (AxisValue :type "Float (single-precision)"))
  (`PrimitiveComponent.AddForce` (`self.Sphere`) (* (`KismetMathLibrary.GetForwardVector` (`KismetMathLibrary.MakeRotator` 0.0 0.0 (.yaw (`self.GetControlRotation`)))) (* AxisValue (`self.MoveForce`))) "None" false))

(event `InputAxis|Move Right / Left`
  (params (AxisValue :type "Float (single-precision)"))
  (`PrimitiveComponent.AddForce` (`self.Sphere`) (* (`KismetMathLibrary.GetRightVector` (`KismetMathLibrary.MakeRotator` 0.0 0.0 (.yaw (`self.GetControlRotation`)))) (* AxisValue (`self.MoveForce`))) "None" false))

(event `Key|LeftShift`
  (params (Key :type "Key Structure"))
  (:`Pressed`
    (set `self.MoveForce` 800000.0))
  (:`Released`
    (set `self.MoveForce` 500000.0)))

(event `self.ReceiveTick`
  (params (DeltaSeconds :type "Float (single-precision)"))
  (bind _downforce (`self.DownForce`))
  (`SceneComponent.K2_SetWorldRotation` (`self.Sphere`) (`KismetMathLibrary.Conv_VectorToRotator` (`KismetMathLibrary.GetForwardVector` (`KismetMathLibrary.MakeRotator` 0.0 0.0 (.yaw (`self.GetControlRotation`))))) false false)
  (`PrimitiveComponent.AddForce` (`self.Sphere`) (`KismetMathLibrary.MakeVector` 0.0 0.0 (`self.UpForce`)) "None" false)
  (`PrimitiveComponent.AddForce` (`self.RightLeg`) (`KismetMathLibrary.MakeVector` 0.0 0.0 _downforce) "None" false)
  (`PrimitiveComponent.AddForce` (`self.LeftLeg`) (`KismetMathLibrary.MakeVector` 0.0 0.0 _downforce) "None" false))

(fn `UserConstructionScript`)