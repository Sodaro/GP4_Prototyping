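; Test character for trying out physical animation on its skeletal mesh.
; A FlipFlop turns physical animation on at BeginPlay, and each R press alternates it off and on through PhysicalAnimComp.
; Tick keeps waking the mesh's rigid body, and a debug print names any component that falls asleep.
; Unconnected leftovers hold a camera line trace and manual physical animation setup that never run.
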(event `Key|LeftMouseButton`
  (params (Key :type "Key Structure")))

(event `Key|R`
  (params (Key :type "Key Structure"))
  (:`Pressed`
    (`/Engine/EditorBlueprintResources/StandardMacros.FlipFlop` :!label _label
      (:`A`
        (`/Game/MartinsTestThings/PhysicalAnimComp.TogglePhysicalAnimation` (`self.PhysicalAnimComp`)))
      (:`B`
        (`/Game/MartinsTestThings/PhysicalAnimComp.UntogglePhysicsAnimation` (`self.PhysicalAnimComp`))))))

(event `self.ReceiveBeginPlay`
  (goto _label))

(event `Key|LeftShift`
  (params (Key :type "Key Structure")))

(event `self.ReceiveTick`
  (params (DeltaSeconds :type "Float (single-precision)"))
  (`PrimitiveComponent.WakeRigidBody` (`self.Mesh`) "None"))

(event `self.Mesh.OnComponentSleep`
  (params (SleepingComponent :type "PrimitiveComponent Object Reference") (BoneName :type Name))
  (`KismetSystemLibrary.PrintString` (`KismetSystemLibrary.GetDisplayName` SleepingComponent)))

(fn `UserConstructionScript`)