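; BP_BigHeadBoy is a test character that experiments with physical animation on its skeletal mesh.
; BeginPlay toggles physical animation on through the PACBigHeadBoy component, while Tick keeps the mesh's rigid body awake and a print reports any sleep event.
; Left Shift sprints, and left click draws a debug visibility trace from the follow camera toward its forward vector scaled from world origin.
; Manual physical-animation setup nodes remain disconnected.
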(event `Key|LeftMouseButton`
  (params (Key :type "Key Structure"))
  (:`Pressed`
    (`KismetSystemLibrary.LineTraceSingle` :`Start` (`SceneComponent.K2_GetComponentLocation` (`self.FollowCamera`)) :`End` (* (`SceneComponent.GetForwardVector` (`self.FollowCamera`)) 1000.0) :`TraceChannel` "TraceTypeQuery1" :`DrawDebugType` "ForDuration")))

(event `Key|R`
  (params (Key :type "Key Structure")))

(event `self.ReceiveBeginPlay`
  (bind _pac_bigheadboy (`self.PAC_BigHeadBoy`))
  (`/Engine/EditorBlueprintResources/StandardMacros.FlipFlop`
    (:`A`
      (`/Game/MartinsTestThings/BigHeadBoy/PAC_BigHeadBoy.TogglePhysicalAnimation` _pac_bigheadboy))
    (:`B`
      (`/Game/MartinsTestThings/BigHeadBoy/PAC_BigHeadBoy.UntogglePhysicsAnimation` _pac_bigheadboy))))

(event `Key|LeftShift`
  (params (Key :type "Key Structure"))
  (bind _charactermovement (`self.CharacterMovement`))
  (:`Pressed`
    (set `CharacterMovementComponent.MaxWalkSpeed` 1000.0 _charactermovement))
  (:`Released`
    (set `CharacterMovementComponent.MaxWalkSpeed` 500.0 _charactermovement)))

(event `self.ReceiveTick`
  (params (DeltaSeconds :type "Float (single-precision)"))
  (`PrimitiveComponent.WakeRigidBody` (`self.Mesh`) "None"))

(event `self.Mesh.OnComponentSleep`
  (params (SleepingComponent :type "PrimitiveComponent Object Reference") (BoneName :type Name))
  (`KismetSystemLibrary.PrintString` (`KismetSystemLibrary.GetDisplayName` SleepingComponent)))

(fn `UserConstructionScript`)